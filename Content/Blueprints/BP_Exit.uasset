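; BP_Exit is a level exit that, while open, sends the player back to the main menu and unlocks the next level.
; A Box overlap checks the IsOpen flag and that the overlapping actor is the third-person character.
; It raises LastLevelUnlocked on the game instance to LevelToUnlock only if that is higher, then removes all widgets and opens L_Menu.
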(event `self.Box.OnComponentBeginOverlap`
  (params (OverlappedComponent :type "PrimitiveComponent Object Reference") (OtherActor :type "Actor Object Reference") (OtherComp :type "PrimitiveComponent Object Reference") (OtherBodyIndex :type Integer) (bFromSweep :type Boolean) (SweepResult :type "HitResult Structure (by ref)"))
  ; If the players owns the key, unlock next level and return to menu
  (if (`self.IsOpen`)
    (cast `/Game/Blueprints/BP_ThirdPersonCharacter` OtherActor)
    (if (< (`/Game/Blueprints/BP_GameInstance.LastLevelUnlocked` (cast `/Game/Blueprints/BP_GameInstance` (`GameplayStatics.GetGameInstance`) :!pure true)) (`self.LevelToUnlock`))
      (`/Game/Blueprints/BP_GameInstance.SetLastLevelUnlocked` (cast `/Game/Blueprints/BP_GameInstance` (`GameplayStatics.GetGameInstance`) :!pure true) (`self.LevelToUnlock`)))
    (`WidgetLayoutLibrary.RemoveAllWidgets`)
    (`GameplayStatics.OpenLevelBySoftObjectPtr` "/Game/Level/L_Menu.L_Menu")))

(fn `UserConstructionScript`)