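; Projectile actor that flies forward and slows any BP_ThirdPersonCharacter it overlaps.
; A Timeline started on BeginPlay offsets it along local X by ProjectileSpeed on each update, without sweep or delta-time scaling, and destroys it on finish.
; On overlapping that character, it destroys itself and passes Damage to the character's LoseSpeed, ignoring all other actors.
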(event `self.ReceiveBeginPlay`
  (`Timeline|Timeline` :!via `PlayFromStart`
    (:`Update`
      (`self.K2_AddActorLocalTransform` (`KismetMathLibrary.Conv_VectorToTransform` (`KismetMathLibrary.MakeVector` (`self.ProjectileSpeed`)))))
    (:`Finished`
      (`self.K2_DestroyActor`))))

(event `self.ReceiveActorBeginOverlap`
  (params (OtherActor :type "Actor Object Reference"))
  (bind _asbp_third_person_character (cast `/Game/Blueprints/BP_ThirdPersonCharacter` OtherActor))
  (`self.K2_DestroyActor`)
  (`/Game/Blueprints/BP_ThirdPersonCharacter.LoseSpeed` _asbp_third_person_character (`self.Damage`)))

(fn `UserConstructionScript`)