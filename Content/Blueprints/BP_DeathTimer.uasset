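; BP_DeathTimer is a level countdown that kills the run and returns to the menu when time runs out.
; On BeginPlay it stretches the DeathTimer timeline to TimeToCompleteLevel via play rate, showing remaining time on the player controller's GameUI each update.
; In the last ten seconds, every update also plays a low-time sound.
; On finish it plays a death sound, slows the player, steps through damage effects, then opens L_Menu.
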(event `self.ReceiveBeginPlay`
  ; Start the death timer, and return to menu when the timer is over
  (`TimelineComponent.SetPlayRate` (`self.DeathTimer`) (/ 1.0 (`self.TimeToCompleteLevel`)))
  (bind (_direction _timer) (`Timeline|DeathTimer`)
    (:`Update`
      (bind _output_get (set `self.Timer` (* _timer (`self.TimeToCompleteLevel`))))
      (bind _output_get_2 (set `self.GameUI` (`/Game/Blueprints/BP_ThirdPersonPlayerController.My Game UI` (cast `/Game/Blueprints/BP_ThirdPersonPlayerController` (`GameplayStatics.GetPlayerController` 0) :!pure true))))
      (bind _returnvalue (- (`self.TimeToCompleteLevel`) _output_get))
      (if (<= _returnvalue 10.0)
        (`GameplayStatics.PlaySound2D` "/Game/Audio/A_LowTimerSound.A_LowTimerSound" 1.0 1.0 0.0 null null))
      (`/Game/UI/WBP_MainUI.ShowTimer` _output_get_2 _returnvalue))
    (:`Finished`
      (`GameplayStatics.PlaySound2D` "/Game/Audio/A_DeathByTime.A_DeathByTime" 1.0 1.0 0.0 null null)
      (`/Game/Blueprints/BP_ThirdPersonCharacter.LoseSpeed` (cast `/Game/Blueprints/BP_ThirdPersonCharacter` (`GameplayStatics.GetPlayerPawn` 0) :!pure true) 1000.0)
      (`/Game/UI/WBP_MainUI.SetDamageEffect` (`/Game/Blueprints/BP_ThirdPersonPlayerController.My Game UI` (cast `/Game/Blueprints/BP_ThirdPersonPlayerController` (`GameplayStatics.GetPlayerController` 0) :!pure true)) 2)
      (`KismetSystemLibrary.Delay` 1.0)
      (`/Game/UI/WBP_MainUI.SetDamageEffect` (`/Game/Blueprints/BP_ThirdPersonPlayerController.My Game UI` (cast `/Game/Blueprints/BP_ThirdPersonPlayerController` (`GameplayStatics.GetPlayerController` 0) :!pure true)) 1)
      (`KismetSystemLibrary.Delay` 1.0)
      (`GameplayStatics.OpenLevelBySoftObjectPtr` "/Game/Level/L_Menu.L_Menu"))))

(fn `UserConstructionScript`)