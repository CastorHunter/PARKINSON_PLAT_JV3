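; BP_SpeakingBox is an interactable actor that shows a line of text to the player through the game UI.
; Its Interract event casts the first player controller to BP_ThirdPersonPlayerController and calls Speak on its MyGameUI.
; The text and display duration come from the box's TextToSay and TimeToShowText variables.
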(event `self.Interract`
  ; Appelle l'event Speak lorsque le joueur interragit avec, en récupérant le texte et le timer convenu
  (`/Game/UI/WBP_MainUI.Speak` (`/Game/Blueprints/BP_ThirdPersonPlayerController.My Game UI` (cast `/Game/Blueprints/BP_ThirdPersonPlayerController` (`GameplayStatics.GetPlayerController` 0) :!pure true)) (`self.TextToSay`) (`self.TimeToShowText`)))

(fn `UserConstructionScript`
  (`parent.UserConstructionScript`))