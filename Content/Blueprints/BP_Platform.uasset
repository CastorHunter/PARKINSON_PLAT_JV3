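; BP_Platform is a moving platform that travels between Start and Goal actors.
; On BeginPlay it snaps to Start and runs a timeline whose play rate derives from TimeToReachGoal.
; Each update sweeps the platform along the line between both positions.
; When within tolerance of the goal and Loop is set, it swaps Start and Goal, waits a second and replays the timeline.
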(event `self.ReceiveBeginPlay`
  ; Move between to positions, waiting one second before changing its goal
  (`self.K2_SetActorLocation` (`self.K2_GetActorLocation` (`self.Start`)))
  (`TimelineComponent.SetPlayRate` (`self.PlatformMovement`) (/ 1.0 (`self.TimeToReachGoal`)))
  (bind (_direction _newtrack_0) (`Timeline|PlatformMovement` :!via `PlayFromStart` :!label _label)
    (:`Update`
      (`self.K2_SetActorLocation` (+ (* (- (`self.K2_GetActorLocation` (`self.Goal`)) (`self.K2_GetActorLocation` (`self.Start`))) (`KismetMathLibrary.FClamp` _newtrack_0 0.0001 1000.0)) (`self.K2_GetActorLocation` (`self.Start`))) true)
      (if (== (`self.K2_GetActorLocation`) (`self.K2_GetActorLocation` (`self.Goal`)) :`ErrorTolerance` 1.0)
        (if (`self.Loop`)
          (set `self.TemporaryGoal` (`self.Goal`))
          (set `self.Goal` (`self.Start`))
          (set `self.Start` (`self.TemporaryGoal`))
          (`KismetSystemLibrary.Delay` 1.0)
          (goto _label :!via `PlayFromStart`))))))

(fn `UserConstructionScript`)