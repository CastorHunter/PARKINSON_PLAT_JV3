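; BP_Key is a collectible key that unlocks a linked gate when the player picks it up.
; On BeginPlay it tints the RectLight of its GateToOpen reference orange.
; On collection it sets the gate's IsOpen flag, destroys itself and switches that light to green.
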(event `self.ReceiveBeginPlay`
  ; Set the gate's color at beginning
  (`LightComponent.SetLightColor` (`/Game/Blueprints/BP_Exit.RectLight` (`self.GateToOpen`)) (struct :`R` 1.0 :`G` 0.267303 :`B` 0.003367 :`A` 1.0) true))

(event `self.OnCollect`
  ; Opens the gate and changes its color when the players collects it
  (set `/Game/Blueprints/BP_Exit.IsOpen` true (`self.GateToOpen`))
  (`self.K2_DestroyActor`)
  (`LightComponent.SetLightColor` (`/Game/Blueprints/BP_Exit.RectLight` (`self.GateToOpen`)) (struct :`R` 0.080353 :`G` 1.0 :`A` 1.0) true))

(fn `UserConstructionScript`
  (`parent.UserConstructionScript`))