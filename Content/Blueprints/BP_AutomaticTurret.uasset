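; Automatic turret actor that tracks the player and fires projectiles at them while they are within its detection range.
; A sphere collision sized from DetectionRange on BeginPlay toggles a Follow flag as the third-person character enters or leaves.
; A timeline whose length is the fire cooldown rotates the turret head toward the player each update.
; On finish it spawns a projectile, Niagara effect and sound, then restarts while following.
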(event `self.ReceiveActorEndOverlap`
  (params (OtherActor :type "Actor Object Reference"))
  ; Stop Following the Player when he leaves the detection range
  (cast `/Game/Blueprints/BP_ThirdPersonCharacter` OtherActor)
  (set `self.Follow` false))

(event `self.ReceiveBeginPlay`
  ; Set the detection range with defined value
  (`SphereComponent.SetSphereRadius` (`self.Sphere1`) (`self.DetectionRange`) true))

(event `self.ReceiveActorBeginOverlap`
  (params (OtherActor :type "Actor Object Reference"))
  ; Follow the player and fire projectiles spaced by a defined time
  (cast `/Game/Blueprints/BP_ThirdPersonCharacter` OtherActor)
  (set `self.Follow` true)
  (`TimelineComponent.SetTimelineLength` (`self.Timeline`) (`self.TurretFireCooldown`))
  (if (`self.Follow`) :!label _label
    (`Timeline|Timeline` :!via `PlayFromStart` :!label _label_2
      (:`Update`
        (if (`self.Follow`)
          (`SceneComponent.K2_SetWorldRotation` (`self.Sphere`) (`KismetMathLibrary.FindLookAtRotation` (`self.K2_GetActorLocation`) (- (`self.K2_GetActorLocation` (`GameplayStatics.GetPlayerCharacter` 0)) (0.0 0.0 45.0))) false false)
          (else
            (goto _label_2 :!via `Stop`))))
      (:`Finished`
        (`|SpawnActorFromClass` "/Game/Blueprints/BP_Projectile.BP_Projectile_C" (`SceneComponent.K2_GetComponentToWorld` (`self.FirePosition`)) "Undefined" "MultiplyWithRoot" null null)
        (`NiagaraFunctionLibrary.SpawnSystemAtLocation` "/Game/VFX/NS_TurretFireEffect.NS_TurretFireEffect" (`SceneComponent.K2_GetComponentLocation` (`self.FirePosition`)) (`SceneComponent.K2_GetComponentRotation` (`self.FirePosition`)))
        (`GameplayStatics.PlaySound2D` "/Game/Audio/A_ProjectileSound.A_ProjectileSound" 1.0 1.0 0.0 null null)
        (goto _label)))))

(fn `UserConstructionScript`)