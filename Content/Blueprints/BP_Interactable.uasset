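; Base-style interactable actor that shows a text prompt when the third-person character enters its box, with an empty Interract event.
; Box overlaps toggle the text and write the controller's CurrentInterctable, apparently inverted: begin overlap clears it to None, end overlap sets it to this actor.
; While visible, the text turns each tick to face the player camera, with roll locked at zero.
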(event `self.ReceiveBeginPlay`
  (`SceneComponent.SetVisibility` (`self.TextRender`) false false))

(event `Interract`)

(event `self.Box.OnComponentEndOverlap`
  (params (OverlappedComponent :type "PrimitiveComponent Object Reference") (OtherActor :type "Actor Object Reference") (OtherComp :type "PrimitiveComponent Object Reference") (OtherBodyIndex :type Integer))
  (cast `/Game/Blueprints/BP_ThirdPersonCharacter` OtherActor)
  (set `/Game/Blueprints/BP_ThirdPersonPlayerController.CurrentInterctable` self (`/Game/Blueprints/BP_FL_Common.GetThirdPersonController`))
  (`SceneComponent.SetVisibility` (`self.TextRender`) false false))

(event `self.Box.OnComponentBeginOverlap`
  (params (OverlappedComponent :type "PrimitiveComponent Object Reference") (OtherActor :type "Actor Object Reference") (OtherComp :type "PrimitiveComponent Object Reference") (OtherBodyIndex :type Integer) (bFromSweep :type Boolean) (SweepResult :type "HitResult Structure (by ref)"))
  (cast `/Game/Blueprints/BP_ThirdPersonCharacter` OtherActor)
  (set `/Game/Blueprints/BP_ThirdPersonPlayerController.CurrentInterctable` null (`/Game/Blueprints/BP_FL_Common.GetThirdPersonController`))
  (`SceneComponent.SetVisibility` (`self.TextRender`) true false))

(event `self.ReceiveTick`
  (params (DeltaSeconds :type "Float (single-precision)"))
  (if (`SceneComponent.IsVisible` (`self.TextRender`))
    (`SceneComponent.K2_SetWorldRotation` (`self.TextRender`) (`KismetMathLibrary.MakeRotator` 0.0 (.pitch (`KismetMathLibrary.FindLookAtRotation` (`SceneComponent.K2_GetComponentLocation` (`self.TextRender`)) (`self.K2_GetActorLocation` (`GameplayStatics.GetPlayerCameraManager` 0)))) (.yaw (`KismetMathLibrary.FindLookAtRotation` (`SceneComponent.K2_GetComponentLocation` (`self.TextRender`)) (`self.K2_GetActorLocation` (`GameplayStatics.GetPlayerCameraManager` 0))))) false false)))

(fn `UserConstructionScript`)